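; Passerby movement Blueprint that walks its owning actor around a fixed rectangular loop in the level.
; Each Tick switches on the CurrentDirection string, which names the current leg, and nudges the owner along one world axis with a swept offset.
; When a hard-coded X or Y bound is passed, it snaps the rotation and switches to the next leg.
; The fixed per-tick step ignores delta time, so speed depends on frame rate.
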(event `self.ReceiveBeginPlay`)

(event `self.ReceiveTick`
  (params (DeltaSeconds :type "Float (single-precision)"))
  (bind _returnvalue (`self.GetOwner`))
  (bind _x (.x (`Actor.K2_GetActorLocation` _returnvalue)))
  (bind _returnvalue_2 (`KismetMathLibrary.FTrunc` (.y (`Actor.K2_GetActorLocation` _returnvalue))))
  (switch `string` (`self.current_direction`)
    (:`x-y-`
      (if (<= _returnvalue_2 1545)
        (`SceneComponent.K2_AddWorldOffset` (`Actor.RootComponent` _returnvalue) (0.0 2.0 0.0) true false)
        (else
          (`Actor.K2_SetActorRotation` _returnvalue (struct :`Yaw` 270.0) false)
          (set `self.current_direction` "x-y+"))))
    (:`x-y+`
      (if (< _x 2028.0)
        (`SceneComponent.K2_AddWorldOffset` (`Actor.RootComponent` _returnvalue) (2.0 0.0 0.0) true false)
        (else
          (`Actor.K2_SetActorRotation` _returnvalue (struct :`Yaw` 180.0) false)
          (set `self.current_direction` "x+y+"))))
    (:`x+y-`
      (if (> _x -1169.0)
        (`SceneComponent.K2_AddWorldOffset` (`Actor.RootComponent` _returnvalue) (-2.0 0.0 0.0) true false)
        (else
          (`Actor.K2_SetActorRotation` _returnvalue (struct) false)
          (set `self.current_direction` "x-y-"))))
    (:`x+y+`
      (if (>= _returnvalue_2 -890)
        (`Actor.K2_AddActorWorldOffset` _returnvalue (0.0 -2.0 0.0) true false)
        (else
          (`Actor.K2_SetActorRotation` _returnvalue (struct :`Yaw` 90.0) false)
          (set `self.current_direction` "x+y-"))))))